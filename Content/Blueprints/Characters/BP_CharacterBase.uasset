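; BP_CharacterBase is a character Blueprint whose event graph toggles the inventory screen from the OpenInventory input action.
; An InventoryCreated flag picks the branch: opening creates a fresh WDB_Inventory widget in the viewport, while closing removes it from its parent.
; Each toggle also switches player controller 0 between game-and-UI input with a visible cursor, focused on the widget, and game-only input with the cursor hidden.
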(event `InputAction|OpenInventory`
  (params (Key :type "Key Structure"))
  (bind _returnvalue (`GameplayStatics.GetPlayerController` 0))
  (:`Pressed`
    (if (`self.bInventoryCreated`)
      (`Widget.RemoveFromParent` (stale _returnvalue_2))
      (set `self.bInventoryCreated` false)
      (set `PlayerController.bShowMouseCursor` false _returnvalue)
      (`WidgetBlueprintLibrary.SetInputMode_GameOnly` _returnvalue)
      (else
        (set `self.bInventoryCreated` true)
        (bind _returnvalue_2 (`|CreateWidget` "/Game/Widgets/InventoryWidget/WDB_Inventory.WDB_Inventory_C" _returnvalue))
        (`UserWidget.AddToViewport` _returnvalue_2 0)
        (`WidgetBlueprintLibrary.SetInputMode_GameAndUIEx` _returnvalue _returnvalue_2)
        (set `PlayerController.bShowMouseCursor` true _returnvalue)))))

(fn `UserConstructionScript`)